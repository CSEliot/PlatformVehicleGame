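; Moving spawner actor that lays a trail of randomly offset platforms, each paired with its own gravity region.
; On a timer, it spawns both in its rotated frame's orientation, sizing the region from platform bounds and pointing gravity against platform up.
; Between spawns it flies forward, randomly starting roll, pitch or yaw turns that stop near ±180 degrees.
; The SpawnPoints grid is built but unused; debug boxes show regions.
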(event EventBeginPlay
  (bind _returnvalue (Game|SpawnActorfromClass "/Game/VehicleAdv/Platform.Platform_C" (Transformation|GetActorTransform) "Undefined" 0 0))
  (bind _output_get (Variables|Default|SetplatformDimensions (* (.BoxExtent (Collision|GetActorBounds _returnvalue false)) 2.0)))
  (Variables|Default|SetspawnPoints (Utilities|Array|MakeArray (Math|Vector|MakeVector 0.0 0.0 0.0) (Math|Vector|MakeVector 0.0 (* (.y _output_get) 1.0) 0.0) (Math|Vector|MakeVector 0.0 (* (.y _output_get) 1.0) (* (.z _output_get) 3.0)) (Math|Vector|MakeVector 0.0 (* (.y _output_get) 1.0) (* (.z _output_get) -3.0)) (Math|Vector|MakeVector 0.0 (* (.y _output_get) -1.0) 0.0) (Math|Vector|MakeVector 0.0 (* (.y _output_get) -1.0) (* (.z _output_get) 3.0)) (Math|Vector|MakeVector 0.0 (* (.y _output_get) -1.0) (* (.z _output_get) -3.0)) (Math|Vector|MakeVector 0.0 0.0 (* (.z _output_get) 3.0)) (Math|Vector|MakeVector 0.0 0.0 (* (.z _output_get) -3.0))))
  (Variables|Default|SetspawnRate 0.6)
  (Variables|Default|SetspawnerSpeed 18.0)
  (Variables|Default|Setmaneuvers (Utilities|Array|MakeArray 0.0 0.0 0.0)))

(event EventTick
  (params (DeltaSeconds :type Float%20%28single-precision%29))
  (bind _returnvalue (Transformation|GetActorTransform))
  (bind _returnvalue_2 (Transformation|GetActorRotation))
  (bind _platformdimensions (Variables|Default|GetplatformDimensions))
  (bind _platformdimensions_2 (Variables|Default|GetplatformDimensions))
  (bind _maneuvers (Variables|Default|Getmaneuvers))
  (bind _returnvalue_3 (* _platformdimensions_2 "0.500000,0.500000,2.000000"))
  (Variables|Default|SetcurrentTime (+ DeltaSeconds (Variables|Default|GetcurrentTime)))
  (if (>= (- (Variables|Default|GetcurrentTime) (Variables|Default|GetspawnTime)) (Variables|Default|GetspawnRate))
    (Variables|Default|SetspawnTime (Variables|Default|GetcurrentTime))
    (bind _output_get (Variables|Default|Settemp (Math|Random|RandomFloatinRange (* (.y _platformdimensions) -3.0) (* (.y _platformdimensions) 3.0))))
    (bind _output_get_2 (Variables|Default|Settemp2 (Math|Random|RandomFloatinRange (* (.z _platformdimensions) -4.0) (* (.z _platformdimensions) 4.0))))
    (bind _returnvalue_4 (Game|SpawnActorfromClass "/Game/VehicleAdv/Platform.Platform_C" (Math|Transform|MakeTransform (+ (.location _returnvalue) (Math|Vector|MakeVector 0.0 _output_get _output_get_2)) (.rotation _returnvalue) (.scale _returnvalue)) "AlwaysSpawn" 0 0))
    (bind _returnvalue_5 (Game|SpawnActorfromClass "/Script/cartest.GravityRegion" (Math|Transform|MakeTransform (+ (+ (.location _returnvalue) (Math|Vector|MakeVector 0.0 _output_get _output_get_2)) (Math|Vector|MakeVector 0.0 0.0 (.z (* (Math|Vector|GetUpVector (.rotation _returnvalue)) (Variables|Default|GetplatformDimensions))))) (.rotation _returnvalue) (.scale _returnvalue)) "AlwaysSpawn" 0 0))
    (Utilities|FlowControl|Sequence
      (:then_0
        (bind _returnvalue_6 (Class|GravityRegion|GetRegion _returnvalue_5))
        (Components|Box|SetBoxExtent _returnvalue_6 _returnvalue_3 true)
        (Rendering|Debug|DrawDebugBox :Center (+ (+ (.location _returnvalue) (Math|Vector|MakeVector 0.0 _output_get _output_get_2)) (Math|Vector|MakeVector 0.0 0.0 (.z (* (Math|Vector|GetUpVector (.rotation _returnvalue)) (Variables|Default|GetplatformDimensions))))) :Extent _returnvalue_3 :Rotation (.rotation _returnvalue) :Duration 1e+01))
      (:then_1
        (bind _returnvalue_7 (Class|GravityRegion|GetGravityArrow _returnvalue_5))
        (Transformation|SetWorldRotation _returnvalue_7 (Math|Conversions|RotationFromXVector (Math|Vector|NegateVector (Transformation|GetActorUpVector _returnvalue_4))) false false))
      (:then_2
        (Class|GravityRegion|SetGravityStrength _returnvalue_5 9.8e+02)))
    (elif (<= (Math|Random|RandomFloat) 0.005)
      (CallFunction|StartRandomManeuver)
      (else
        (Transformation|SetActorRotation (Math|Rotator|CombineRotators (Transformation|GetActorRotation) (Math|Rotator|MakeRotator (Utilities|Array|Get(acopy) _maneuvers) (Utilities|Array|Get(acopy) _maneuvers 1) (Utilities|Array|Get(acopy) _maneuvers 2))))
        (Utilities|FlowControl|Sequence
          (:then_0
            (CallFunction|CheckEndManeuver 0 (.roll _returnvalue_2)))
          (:then_1
            (CallFunction|CheckEndManeuver 1 (.pitch _returnvalue_2)))
          (:then_2
            (CallFunction|CheckEndManeuver 2 (.yaw _returnvalue_2)))
          (:then_3
            (Transformation|SetActorLocation (+ (Transformation|GetActorLocation) (* (Transformation|GetActorForwardVector) (Variables|Default|GetspawnerSpeed))) false false)))))))

(fn ConstructionScript)

(fn StartRandomManeuver
  (bind _maneuvers (Variables|Default|Getmaneuvers))
  (bind _returnvalue (Utilities|Array|Length _maneuvers))
  (bind _returnvalue_2 (- _returnvalue 1))
  (bind _returnvalue_3 (Math|Random|RandomIntegerinRange 0 _returnvalue_2))
  (if (== (Utilities|Array|Get(acopy) _maneuvers _returnvalue_3) 0.0)
    (Utilities|Array|SetArrayElem _maneuvers _returnvalue_3 (Math|Random|RandomFloatinRange -0.4 0.4)))
  (return))

(fn CheckEndManeuver
  (params (Index :type Integer) (A :type Float%20%28single-precision%29))
  (if (Math|Float|NearlyEqual(Float) (Math|Float|Absolute(Float) A) 1.8e+02 1.0)
    (Utilities|Array|SetArrayElem (Variables|Default|Getmaneuvers) Index (Math|Float|MakeLiteralFloat 0.0)))
  (return))